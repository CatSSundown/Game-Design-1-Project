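; BP_Key is a collectible key pickup actor that the player gathers by walking into it.
; On box collision overlap it casts the other actor to BP_ThirdPersonCharacterCustom and increments that character's KeyCount.
; It then prints the new count, plays a key sound at a location and destroys itself.
; Debug strings report spawning, pickup and failed casts.
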(event OnComponentBeginOverlap(BoxCollision)
  (params (OverlappedComponent :type Primitive%20Component%20Object%20Reference) (OtherActor :type Actor%20Object%20Reference) (OtherComp :type Primitive%20Component%20Object%20Reference) (OtherBodyIndex :type Integer) (bFromSweep :type Boolean) (SweepResult :type Hit%20Result%20Structure%20%28by%20ref%29))
  (bind _asbp_third_person_character_custom (Utilities|Casting|CastToBP_ThirdPersonCharacterCustom OtherActor)
    (:then
      (Development|PrintString "Key has been Overlapped by Player" true true "(R=0.000000,G=0.660000,B=1.000000,A=1.000000)" 5.0)
      (Variables|/Game/Blueprints/BP_ThirdPersonCharacterCustom.BP_ThirdPersonCharacterCustom_C|SetKey%20Count _asbp_third_person_character_custom (+ (Variables|/Game/Blueprints/BP_ThirdPersonCharacterCustom.BP_ThirdPersonCharacterCustom_C|GetKey%20Count _asbp_third_person_character_custom) 1)) ; Set Key Count
      (Development|PrintString (Utilities|String|Append "The Player has " (Utilities|String|ToString(Integer) (Variables|/Game/Blueprints/BP_ThirdPersonCharacterCustom.BP_ThirdPersonCharacterCustom_C|GetKey%20Count _asbp_third_person_character_custom)) " key(s)."))
      (Audio|PlaySoundatLocation "/Game/Sounds/SFX/Keys.Keys" "0, 0, 0" "0, 0, 0" 2.0 1.0 0.0 0 0 0 0)
      (Actor|DestroyActor) ; Destroy this key
    )
    (:CastFailed
      (Development|PrintString "Key Player Cast Failed" true true "(R=0.875000,G=0.000000,B=0.029306,A=1.000000)"))))

(event EventBeginPlay
  (Development|PrintString "This Key Exists!" true true "(R=0.989389,G=0.130208,B=1.000000,A=1.000000)"))

(fn ConstructionScript)