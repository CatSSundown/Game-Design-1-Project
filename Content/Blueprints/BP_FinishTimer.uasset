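; BP_FinishTimer is a finish-line trigger that reports lap times for the custom third-person character.
; When that character overlaps OverlapBox, it prints the real seconds elapsed since the stored timestamp, rounded to one decimal, then resets the timestamp.
; BeginPlay creates a W_FinishLineTimer widget but does not add it to the viewport or feed it the time.
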(event OnComponentBeginOverlap(OverlapBox)
  (params (OverlappedComponent :type Primitive%20Component%20Object%20Reference) (OtherActor :type Actor%20Object%20Reference) (OtherComp :type Primitive%20Component%20Object%20Reference) (OtherBodyIndex :type Integer) (bFromSweep :type Boolean) (SweepResult :type Hit%20Result%20Structure%20%28by%20ref%29))
  (Utilities|Casting|CastToBP_ThirdPersonCharacterCustom OtherActor)
  (Development|PrintString (Utilities|String|Append "That Lap Took " (Utilities|String|ToString(Text) (Utilities|Text|ToText(Float) (- (Utilities|Time|GetRealTimeSeconds) (Variables|Default|GetLast%20TImestamp)) "HalfToEven" false true 1 324 0 1)) "Seconds!"))
  (Variables|Default|SetLast%20TImestamp (Utilities|Time|GetRealTimeSeconds)))

(event EventBeginPlay
  (UserInterface|CreateWidget "/Game/Widgets/W_FinishLineTimer.W_FinishLineTimer_C"))

(event Collision|EventActorBeginOverlap
  (params (OtherActor :type Actor%20Object%20Reference)))

(event EventTick
  (params (DeltaSeconds :type Float%20%28single-precision%29)))

(fn ConstructionScript)